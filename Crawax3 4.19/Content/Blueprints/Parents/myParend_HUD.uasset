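; Parent HUD Blueprint that draws a rectangular screen selection zone.
; SetSelectZoneOrigin stores the start corner, while SetSelectBox supplies the end corner and opens a Gate that StopSelectBox closes.
; While the Gate is open, DrawHUD compares both corners on X and Y and picks one of four DrawRect calls, keeping width and height positive in any direction.
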(event Custom|StopSelectBox
  (bind _selectzoneorigin (Variables|Default|GetSelectZoneOrigin))
  (bind _selectzoneorigin_2 (Variables|Default|GetSelectZoneOrigin))
  (bind _selectzoneorigin_3 (Variables|Default|GetSelectZoneOrigin))
  (bind _selectzoneorigin_4 (Variables|Default|GetSelectZoneOrigin))
  (bind _selectzoneorigin_5 (Variables|Default|GetSelectZoneOrigin))
  (bind (_x _y) (Math|Vector2D|BreakVector2D _selectzoneorigin))
  (bind (_x_2 _y_2) (Math|Vector2D|BreakVector2D _selectzoneorigin_2))
  (bind (_x_3 _y_3) (Math|Vector2D|BreakVector2D _selectzoneorigin_5))
  (bind (_x_4 _y_4) (Math|Vector2D|BreakVector2D _selectzoneorigin_4))
  (bind (_x_5 _y_5) (Math|Vector2D|BreakVector2D _selectzoneorigin_3))
  (Utilities|FlowControl|Gate true) ; enters at Close
)

(event Custom|SetSelectZoneOrigin
  (params (SelectZoneOrigin :type Vector%202D%20Structure))
  (Variables|Default|SetSelectZoneOrigin SelectZoneOrigin))

(event Custom|SetSelectBox
  (params (SelectBoxPosEnd :type Vector%202D%20Structure))
  (bind (_x _y) (Math|Vector2D|BreakVector2D SelectBoxPosEnd))
  (bind (_x_2 _y_2) (Math|Vector2D|BreakVector2D SelectBoxPosEnd))
  (bind (_x_3 _y_3) (Math|Vector2D|BreakVector2D SelectBoxPosEnd))
  (bind (_x_4 _y_4) (Math|Vector2D|BreakVector2D SelectBoxPosEnd))
  (bind (_x_5 _y_5) (Math|Vector2D|BreakVector2D SelectBoxPosEnd))
  (bind _selectzoneorigin (Variables|Default|GetSelectZoneOrigin))
  (bind _selectzoneorigin_2 (Variables|Default|GetSelectZoneOrigin))
  (bind _selectzoneorigin_3 (Variables|Default|GetSelectZoneOrigin))
  (bind _selectzoneorigin_4 (Variables|Default|GetSelectZoneOrigin))
  (bind _selectzoneorigin_5 (Variables|Default|GetSelectZoneOrigin))
  (bind (_x_6 _y_6) (Math|Vector2D|BreakVector2D _selectzoneorigin))
  (bind (_x_7 _y_7) (Math|Vector2D|BreakVector2D _selectzoneorigin_2))
  (bind (_x_8 _y_8) (Math|Vector2D|BreakVector2D _selectzoneorigin_5))
  (bind (_x_9 _y_9) (Math|Vector2D|BreakVector2D _selectzoneorigin_4))
  (bind (_x_10 _y_10) (Math|Vector2D|BreakVector2D _selectzoneorigin_3))
  (bind _returnvalue (< _y_6 _y))
  (Utilities|FlowControl|Gate true) ; enters at Open
)

(event EventDrawHUD
  (params (SizeX :type Integer) (SizeY :type Integer))
  (bind _selectzoneorigin (Variables|Default|GetSelectZoneOrigin))
  (bind _selectzoneorigin_2 (Variables|Default|GetSelectZoneOrigin))
  (bind _selectzoneorigin_3 (Variables|Default|GetSelectZoneOrigin))
  (bind _selectzoneorigin_4 (Variables|Default|GetSelectZoneOrigin))
  (bind _selectzoneorigin_5 (Variables|Default|GetSelectZoneOrigin))
  (bind (_x _y) (Math|Vector2D|BreakVector2D _selectzoneorigin))
  (bind (_x_2 _y_2) (Math|Vector2D|BreakVector2D _selectzoneorigin_2))
  (bind (_x_3 _y_3) (Math|Vector2D|BreakVector2D _selectzoneorigin_5))
  (bind (_x_4 _y_4) (Math|Vector2D|BreakVector2D _selectzoneorigin_4))
  (bind (_x_5 _y_5) (Math|Vector2D|BreakVector2D _selectzoneorigin_3))
  (Utilities|FlowControl|Gate true
    (:Exit
      (if (< _x (.X (Math|Vector2D|BreakVector2D (stale Custom|SetSelectBox SelectBoxPosEnd))))
        (if (< _y (.Y (Math|Vector2D|BreakVector2D (stale Custom|SetSelectBox SelectBoxPosEnd))))
          ;[1 1 1] X>/Y>
          (HUD|DrawRect (Variables|Default|GetSelectZoneColor) _x_3 _y_3 (- (.X (Math|Vector2D|BreakVector2D (stale Custom|SetSelectBox SelectBoxPosEnd))) _x_3) (- (.Y (Math|Vector2D|BreakVector2D (stale Custom|SetSelectBox SelectBoxPosEnd))) _y_3) :!pinned true) ; X>/Y>
          (else
            ;[1 1 1] X>/Y<
            (HUD|DrawRect (Variables|Default|GetSelectZoneColor) _x_4 (.Y (Math|Vector2D|BreakVector2D (stale Custom|SetSelectBox SelectBoxPosEnd))) (- (.X (Math|Vector2D|BreakVector2D (stale Custom|SetSelectBox SelectBoxPosEnd))) _x_4) (- _y_4 (.Y (Math|Vector2D|BreakVector2D (stale Custom|SetSelectBox SelectBoxPosEnd)))) :!pinned true) ; X>/Y<
          ))
        (elif (< _y (.Y (Math|Vector2D|BreakVector2D (stale Custom|SetSelectBox SelectBoxPosEnd))))
          ;[1 1 1] X</Y>
          (HUD|DrawRect (Variables|Default|GetSelectZoneColor) (.X (Math|Vector2D|BreakVector2D (stale Custom|SetSelectBox SelectBoxPosEnd))) _y_5 (- _x_5 (.X (Math|Vector2D|BreakVector2D (stale Custom|SetSelectBox SelectBoxPosEnd)))) (- (.Y (Math|Vector2D|BreakVector2D (stale Custom|SetSelectBox SelectBoxPosEnd))) _y_5) :!pinned true) ; X</Y>
          (else
            ;[1 1 1] Y</X<
            (HUD|DrawRect (Variables|Default|GetSelectZoneColor) (.X (Math|Vector2D|BreakVector2D (stale Custom|SetSelectBox SelectBoxPosEnd))) (.Y (Math|Vector2D|BreakVector2D (stale Custom|SetSelectBox SelectBoxPosEnd))) (- _x_2 (.X (Math|Vector2D|BreakVector2D (stale Custom|SetSelectBox SelectBoxPosEnd)))) (- _y_2 (.Y (Math|Vector2D|BreakVector2D (stale Custom|SetSelectBox SelectBoxPosEnd)))) :!pinned true) ; Y</X<
          ))))))

(fn ConstructionScript)