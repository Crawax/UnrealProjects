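; Parent camera pawn with reusable functions for planar movement, spring-arm zoom and yaw rotation.
; ApplyMovement offsets the actor relative to its rotation without sweep, dampens diagonal speed and scales speed with zoom, so close views pan slower.
; ApplyZoom eases arm length within min/max limits, starting from a default set on BeginPlay.
; ApplyRotation eases yaw by the clamped input times rotation speed and ratio; no input is bound here.
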(event EventBeginPlay
  (Variables|/Script/Engine.SpringArmComponent|SetTargetArmLength (Variables|Default|GetSpringArm) (Variables|SpringArm|GetSprintArmLenghtDefault)))

(fn ConstructionScript)

(fn ApplyMovement
  (params (MovementRatio :type Vector%202D%20Structure))
  (bind _returnvalue (Transformation|GetActorLocation))
  (bind _returnvalue_2 (Transformation|GetActorRotation))
  (bind _sprintarmlenghtmax (Variables|SpringArm|GetSprintArmLenghtMax))
  (bind _sprintarmlenghtmin (Variables|SpringArm|GetSprintArmLenghtMin))
  (bind _springarm (Variables|Default|GetSpringArm))
  (bind _sprintarmlenghtmin_2 (Variables|SpringArm|GetSprintArmLenghtMin))
  (bind _movementspeed (Variables|Movement|GetMovementSpeed))
  (bind _returnvalue_3 (- _sprintarmlenghtmax _sprintarmlenghtmin))
  (bind _targetarmlength (Variables|/Script/Engine.SpringArmComponent|GetTargetArmLength _springarm))
  (bind _returnvalue_4 (- _targetarmlength _sprintarmlenghtmin_2))
  (bind _returnvalue_5 (/ _returnvalue_4 _returnvalue_3))
  (bind _returnvalue_6 (Math|Float|Clamp(Float) _returnvalue_5 0.3))
  (bind _returnvalue_7 (* _movementspeed _returnvalue_6))
  (bind _returnvalue_8 (* (.y MovementRatio) _returnvalue_7))
  (bind _returnvalue_9 (* (.x MovementRatio) _returnvalue_7))
  (bind _returnvalue_10 (Math|Transform|TransformDirection (Math|Transform|MakeTransform _returnvalue _returnvalue_2 "1,1,1") (Math|Vector|MakeVector _returnvalue_9 _returnvalue_8 0.0)))
  (bind (_x _y) (Math|Vector|BreakVector _returnvalue_10))
  (if (!= (.x MovementRatio) 0.0)
    (Transformation|SetActorLocation (Math|Interpolation|VInterpTo _returnvalue (+ _returnvalue (/ _returnvalue_10 (Math|Float|Clamp(Float) (/ (+ (Math|Float|Absolute(Float) _x) (Math|Float|Absolute(Float) _y)) _returnvalue_7) 1.0 2.0))) (Utilities|Time|GetWorldDeltaSeconds) 1.0) false false :!label _label)
    (elif (!= (.y MovementRatio) 0.0)
      (goto _label))))

(fn ApplyZoom
  (params (ZoomValue :type Float%20%28single-precision%29))
  (if (!= ZoomValue 0.0)
    (Variables|/Script/Engine.SpringArmComponent|SetTargetArmLength (Variables|Default|GetSpringArm) (Math|Float|Clamp(Float) (Math|Interpolation|FInterpTo (Variables|/Script/Engine.SpringArmComponent|GetTargetArmLength (Variables|Default|GetSpringArm)) (+ (Variables|/Script/Engine.SpringArmComponent|GetTargetArmLength (Variables|Default|GetSpringArm)) (* ZoomValue (Variables|SpringArm|GetSpringArmZoomSpeed))) (Utilities|Time|GetWorldDeltaSeconds) 5.0) (Variables|SpringArm|GetSprintArmLenghtMin) (Variables|SpringArm|GetSprintArmLenghtMax)))))

(fn ApplyRotation
  (params (RotationValue :type Float%20%28single-precision%29))
  (bind _returnvalue (Transformation|GetActorRotation))
  (bind _returnvalue_2 (Transformation|GetActorRotation))
  (bind (_roll _pitch _yaw) (Math|Rotator|BreakRotator _returnvalue_2))
  (bind (_roll_2 _pitch_2 _yaw_2) (Math|Rotator|BreakRotator _returnvalue))
  (if (!= RotationValue 0.0)
    (if (> RotationValue 0.0)
      (Transformation|SetActorRotation (Math|Rotator|MakeRotator _roll_2 _pitch_2 (Math|Interpolation|FInterpTo _yaw_2 (+ _yaw_2 (* (Math|Float|Clamp(Float) RotationValue) (* (Variables|Rotation|GetRotationSpeed) (Variables|Rotation|GetRotationSpeedRatio)))) (Utilities|Time|GetWorldDeltaSeconds) 2.0)))
      (else
        (Transformation|SetActorRotation (Math|Rotator|MakeRotator _roll _pitch (Math|Interpolation|FInterpTo _yaw (+ _yaw (* (Math|Float|Clamp(Float) RotationValue -1.0 0.0) (* (Variables|Rotation|GetRotationSpeed) (Variables|Rotation|GetRotationSpeedRatio)))) (Utilities|Time|GetWorldDeltaSeconds) 2.0)))))))